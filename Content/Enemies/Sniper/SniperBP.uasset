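; Sniper enemy Blueprint that fires projectiles at the player and shows its state through a colored vision cone.
; Construction binds the modular skeletal armor and body parts to the main mesh pose and snaps the gun to the GripPoint socket.
; FireProjectile reads TargetActor from the blackboard and leads the moving player by velocity scaled with distance.
; ChangeColor tints the cone for normal, red or stunned states; StunAI is an empty stub.
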(fn ConstructionScript
  (Class|SkinnedMeshComponent|SetMasterPoseComponent (Variables|Default|GetSK_Etasphera31_Arm_thumb_03_r) (Variables|Character|GetMesh) false)
  (Transformation|AttachComponentToComponent (Variables|Default|GetGun) (Variables|Character|GetMesh) "GripPoint" "SnapToTarget" "KeepRelative" "SnapToTarget" true))

(fn FireProjectile
  (bind _firing_point (Variables|Default|GetFiring%20Point))
  (bind _returnvalue (Transformation|GetWorldLocation _firing_point))
  (bind _asfirst_person_character (Utilities|Casting|CastToFirstPersonCharacter (AI|Components|Blackboard|GetValueasObject (AI|GetBlackboard 0) (Utilities|Name|MakeLiteralName "TargetActor"))))
  (Game|SpawnActorfromClass "/Game/Enemies/Sniper/EnemyProjectile.EnemyProjectile_C" (Math|Transform|MakeTransform _returnvalue (Math|Rotator|FindLookatRotation _returnvalue (+ (Transformation|GetWorldLocation (Variables|/Script/Engine.Character|GetMesh _asfirst_person_character)) (* (Transformation|GetVelocity _asfirst_person_character) (/ (Transformation|GetDistanceTo _asfirst_person_character) 5e+03))))) "Undefined" 0 0))

(fn StunAI)

(fn ChangeColor
  (params (NewParam :type String))
  (bind _visioncone (Variables|Default|GetVisionCone))
  (switch string NewParam
    (:Default
      (bind _returnvalue (Rendering|Material|CreateDynamicMaterialInstance _visioncone 0 "/Game/Enemies/AI_Helper/VisionCone.VisionCone" "None" :!class /Script/Engine.PrimitiveComponent :!label _label))
      (Rendering|Material|SetVectorParameterValue _returnvalue "BaseColor" "(R=0.239216,G=0.239216,B=0.239216,A=1.000000)" :!class /Script/Engine.MaterialInstanceDynamic)
      (Rendering|Material|SetVectorParameterValue _returnvalue "EmissiveColor" "(R=0.239216,G=0.239216,B=0.239216,A=1.000000)" :!class /Script/Engine.MaterialInstanceDynamic))
    (:Red
      (bind _returnvalue_2 (Rendering|Material|CreateDynamicMaterialInstance _visioncone 0 "/Game/Enemies/AI_Helper/VisionCone.VisionCone" "None" :!class /Script/Engine.PrimitiveComponent))
      (Rendering|Material|SetVectorParameterValue _returnvalue_2 "BaseColor" "(R=0.239216,G=0.000000,B=0.007843,A=1.000000)" :!class /Script/Engine.MaterialInstanceDynamic)
      (Rendering|Material|SetVectorParameterValue _returnvalue_2 "EmissiveColor" "(R=0.239216,G=0.000000,B=0.007843,A=1.000000)" :!class /Script/Engine.MaterialInstanceDynamic))
    (:Normal
      (goto _label))
    (:Stunned
      (bind _returnvalue_3 (Rendering|Material|CreateDynamicMaterialInstance _visioncone 0 "/Game/Enemies/AI_Helper/VisionCone.VisionCone" "None" :!class /Script/Engine.PrimitiveComponent))
      (Rendering|Material|SetVectorParameterValue _returnvalue_3 "BaseColor" "(R=0.035294,G=0.203922,B=0.239216,A=1.000000)" :!class /Script/Engine.MaterialInstanceDynamic)
      (Rendering|Material|SetVectorParameterValue _returnvalue_3 "EmissiveColor" "(R=0.035294,G=0.203922,B=0.239216,A=1.000000)" :!class /Script/Engine.MaterialInstanceDynamic))))