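; Chaser enemy that deals continuous contact damage to the first-person player character.
; Entering its PlayerDamager volume starts a fast looping timer that applies damage, and leaving clears it.
; FireProjectile spawns an EnemyProjectile at the actor's location and rotation.
; ChangeColor tints the vision cone for normal, red or stunned states through a new dynamic material instance on each call; neither function is called within this Blueprint.
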(event OnComponentBeginOverlap(PlayerDamager)
  (params (OverlappedComponent :type Primitive%20Component%20Object%20Reference) (OtherActor :type Actor%20Object%20Reference) (OtherComp :type Primitive%20Component%20Object%20Reference) (OtherBodyIndex :type Integer) (bFromSweep :type Boolean) (SweepResult :type Hit%20Result%20Structure%20%28by%20ref%29))
  (bind _asfirst_person_character (Utilities|Casting|CastToFirstPersonCharacter OtherActor))
  (Variables|Default|SetAs%20First%20Person%20Character _asfirst_person_character)
  (bind _returnvalue (Utilities|Time|SetTimerbyEvent (delegate Custom|DamagePlayer) 0.01 true))
  (Variables|Default|SetTimerRef _returnvalue))

(event OnComponentEndOverlap(PlayerDamager)
  (params (OverlappedComponent :type Primitive%20Component%20Object%20Reference) (OtherActor :type Actor%20Object%20Reference) (OtherComp :type Primitive%20Component%20Object%20Reference) (OtherBodyIndex :type Integer))
  (Utilities|Casting|CastToFirstPersonCharacter OtherActor)
  (Utilities|Time|ClearandInvalidateTimerbyHandle (Variables|Default|GetTimerRef)))

(event Custom|DamagePlayer
  (Game|Damage|ApplyDamage (Variables|Default|GetAs%20First%20Person%20Character) 1.0 0 0))

(fn ConstructionScript)

(fn FireProjectile
  (bind _returnvalue (Transformation|GetActorTransform))
  (Game|SpawnActorfromClass "/Game/Enemies/Sniper/EnemyProjectile.EnemyProjectile_C" (Math|Transform|MakeTransform (.location _returnvalue) (.rotation _returnvalue)) "Undefined" 0 0))

(fn ChangeColor
  (params (NewParam :type String))
  (bind _visioncone (Variables|Default|GetVisionCone))
  (switch string NewParam
    (:Default
      (bind _returnvalue (Rendering|Material|CreateDynamicMaterialInstance _visioncone 0 "/Game/Enemies/AI_Helper/VisionCone.VisionCone" "None" :!class /Script/Engine.PrimitiveComponent :!label _label))
      (Rendering|Material|SetVectorParameterValue _returnvalue "BaseColor" "(R=0.239216,G=0.239216,B=0.239216,A=1.000000)" :!class /Script/Engine.MaterialInstanceDynamic))
    (:Red
      (bind _returnvalue_2 (Rendering|Material|CreateDynamicMaterialInstance _visioncone 0 "/Game/Enemies/AI_Helper/VisionCone.VisionCone" "None" :!class /Script/Engine.PrimitiveComponent))
      (Rendering|Material|SetVectorParameterValue _returnvalue_2 "BaseColor" "(R=0.239216,G=0.000000,B=0.007843,A=1.000000)" :!class /Script/Engine.MaterialInstanceDynamic))
    (:Normal
      (goto _label))
    (:Stunned
      (bind _returnvalue_3 (Rendering|Material|CreateDynamicMaterialInstance _visioncone 0 "/Game/Enemies/AI_Helper/VisionCone.VisionCone" "None" :!class /Script/Engine.PrimitiveComponent))
      (Rendering|Material|SetVectorParameterValue _returnvalue_3 "BaseColor" "(R=0.036840,G=0.205735,B=0.239216,A=1.000000)" :!class /Script/Engine.MaterialInstanceDynamic))))