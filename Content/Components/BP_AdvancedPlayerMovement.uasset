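; Actor component that gives a character wall running, wall jumps, double jumps and an air-or-ground dash.
; A looping timer traces right and left for near-vertical walls while falling, launches the character along them and eases gravity toward a target.
; Ending a run restores gravity and briefly suppresses re-attachment, while Tick rolls the camera away from the wall.
; Dash fakes a timeline with a timer and Tick gate, applying eased, swept offsets.
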(event Custom|Initialize
  (params (Character :type Character%20Object%20Reference))
  (bind _output_get (Variables|Default|SetCharacter Character))
  (bind _output_get_2 (Variables|Default|SetCharacter%20Movement (Variables|/Script/Engine.Character|GetCharacterMovement _output_get)))
  (Variables|Default|SetDefaultGravity (Variables|/Script/Engine.CharacterMovementComponent|GetGravityScale _output_get_2))
  (Utilities|Time|SetTimerbyEvent (delegate Custom|WallRunUpdateEvent) 0.02 true))

(event Custom|LandEvent
  (CallFunction|WallRunEnd 0.0)
  (Variables|Default|SetWallRunSuppressed? false)
  (Variables|Default|SetCanDoubleJump? true))

(event Custom|JumpEvent
  (params (DoubleJumpVelocity :type Vector))
  ;[1 1 1] Jumping (Including jumping off walls & double jumping)
  (bind _haswalljumped_ (CallFunction|WallRunJump))
  (if (Math|Boolean|ANDBoolean (not _haswalljumped_) (not (Character|CanJump (Variables|Default|GetCharacter))) (Variables|Default|GetCanDoubleJump?))
    (Variables|Default|SetCanDoubleJump? false)
    (Variables|Default|SetDashCancelled? true)
    (Character|LaunchCharacter (Variables|Default|GetCharacter) DoubleJumpVelocity false true)))

(event Custom|WallRunUpdateEvent
  (if (not (Variables|Default|GetWallRunSuppressed?))
    (CallFunction|WallRunUpdate)))

(event Custom|ResetWallRunSuppression
  (Utilities|Time|ClearTimerbyFunctionName 0 "ResetWallRunSuppression")
  (Variables|Default|SetWallRunSuppressed? false))

(event Custom|DashEvent
  (params (DashDirection :type Vector))
  ;[1 1 1] Dash Code (Includes sloppy workaround for lack of timeline functionality in Actor Components)
  (Variables|Default|SetDash%20Direction DashDirection)
  (if (Variables|Default|GetCanDash?)
    (Variables|Default|SetCanDash? false)
    (Variables|Default|SetDashCancelled? false)
    (CallFunction|UE5JustCouldntAddTimelinestoActorCompsHuh)))

(event Custom|Finished
  ;[1 1 1] Dash Code (Includes sloppy workaround for lack of timeline functionality in Actor Components)
  (Utilities|Time|ClearandInvalidateTimerbyHandle (Variables|Default|GetTimer%20Handle))
  (Utilities|FlowControl|Sequence
    (:then_0
      (Utilities|FlowControl|Gate true) ; enters at Close
    )
    (:then_1
      (Utilities|FlowControl|Delay 1.0)
      (Variables|Default|SetCanDash? true))))

(event Custom|UE5JustCouldntAddTimelinesToActorCompsHuh
  (bind _dashduration (Variables|Default|GetDashDuration))
  ;[1 1 1] Dash Code (Includes sloppy workaround for lack of timeline functionality in Actor Components)
  (bind _returnvalue (Utilities|Time|SetTimerbyEvent (delegate Custom|Finished) _dashduration))
  (bind _output_get (Variables|Default|SetTimer%20Handle _returnvalue))
  (Utilities|FlowControl|Gate true) ; enters at Open
)

(event EventTick
  (params (DeltaSeconds :type Float%20%28single-precision%29))
  ;[1 1 1] Dash Code (Includes sloppy workaround for lack of timeline functionality in Actor Components)
  (CallFunction|CameraTick)
  (Utilities|FlowControl|Gate true
    (:Exit
      (Character|LaunchCharacter (Variables|Default|GetCharacter) "0, 0, 0" false (not (Variables|Default|GetDashCancelled?)))
      (Transformation|AddWorldOffset (Variables|/Script/Engine.Actor|GetRootComponent (Variables|Default|GetCharacter)) (* (Variables|Default|GetDash%20Direction) (Math|Interpolation|Ease "EaseOut" (Math|Float|MapRangeUnclamped (Class|KismetSystemLibrary|GetTimerElapsedTimeHandle (stale Custom|UE5JustCouldntAddTimelinesToActorCompsHuh _output_get)) 0.0 (Variables|Default|GetDashDuration) 0.0 1.0) (Variables|Default|GetDashSpeed) 0.0 1.0)) true false))))

(fn WallRunUpdate
  (bind _onwall (CallFunction|WallRunMovement (Transformation|GetActorLocation (Variables|Default|GetCharacter)) (.Right (Utilities|WallRunEndVectors)) -1.0))
  (if _onwall
    (bind _output_get (Variables|Default|SetWallRunning? true))
    (Variables|Default|SetWallRunningR? _output_get)
    (Variables|Default|SetWallRunningL? false)
    (Variables|/Script/Engine.CharacterMovementComponent|SetGravityScale (Variables|Default|GetCharacter%20Movement) (Math|Interpolation|FInterpTo (Variables|/Script/Engine.CharacterMovementComponent|GetGravityScale (Variables|Default|GetCharacter%20Movement)) (Variables|Default|GetWallRunTargetGravity) (Utilities|Time|GetWorldDeltaSeconds) 1e+01) :!label _label)
    (Variables|Default|SetCanDoubleJump? false)
    (elif (Variables|Default|GetWallRunningR?)
      (CallFunction|WallRunEnd 1.0)
      (else
        (bind _onwall_2 (CallFunction|WallRunMovement (Transformation|GetActorLocation (Variables|Default|GetCharacter)) (.Left (Utilities|WallRunEndVectors)) 1.0))
        (if _onwall_2
          (Variables|Default|SetWallRunning? true)
          (Variables|Default|SetWallRunningR? false)
          (Variables|Default|SetWallRunningL? true)
          (goto _label)
          (else
            (CallFunction|WallRunEnd 1.0)))))))

(fn WallRunMovement
  (params (Start :type Vector) (End :type Vector) (WallRunDirection :type Float%20%28single-precision%29))
  (bind _outhit (Collision|LineTraceByChannel Start End "TraceTypeQuery1" false 0 "None"))
  (if (.bblockinghit _outhit)
    (if (and (.ReturnValue (Utilities|ValidWallRunVector? (.normal _outhit))) (AI|Components|NavMovement|IsFalling (Variables|Default|GetCharacter%20Movement)))
      (Variables|Default|SetWallRunNormal (.OutVec (Utilities|ValidWallRunVector? (.normal _outhit))))
      (Character|LaunchCharacter (Variables|Default|GetCharacter) (Utilities|PlayertoWallVector) false false) ; Stick to wall
      (Character|LaunchCharacter (Variables|Default|GetCharacter) (* (Math|Vector|CrossProduct (Variables|Default|GetWallRunNormal) "0, 0,1.000000") (* (Variables|Default|GetWallRunSpeed) WallRunDirection)) true (not (Variables|Default|GetWallRunGravity?))) ; Move forward
      (return true)
      (else
        (return false)))
    (else
      (return false))))

(fn WallRunEnd
  (params (ResetTime :type Float%20%28single-precision%29))
  (if (Variables|Default|GetWallRunning?)
    (Variables|Default|SetWallRunning? false)
    (Variables|Default|SetWallRunningL? false)
    (Variables|Default|SetWallRunningR? false)
    (Variables|/Script/Engine.CharacterMovementComponent|SetGravityScale (Variables|Default|GetCharacter%20Movement) (Variables|Default|GetDefaultGravity))
    (Variables|Default|SetCanDoubleJump? true)
    (CallFunction|SuppressWallRun ResetTime)))

(fn SuppressWallRun
  (params (Delay :type Float%20%28single-precision%29))
  (Variables|Default|SetWallRunSuppressed? true)
  (Utilities|Time|SetTimerbyFunctionName 0 "ResetWallRunSuppression" Delay))

(fn CameraTick
  (if (Variables|Default|GetWallRunningL?)
    (CallFunction|CameraTilt 15.0)
    (elif (Variables|Default|GetWallRunningR?)
      (CallFunction|CameraTilt -15.0)
      (else
        (CallFunction|CameraTilt 0.0)))))

(fn CameraTilt
  (params (Target%20X%20%28Roll%29 :type Float%20%28single-precision%29))
  (bind _character (Variables|Default|GetCharacter))
  (bind _returnvalue (Pawn|GetController _character))
  (bind _returnvalue_2 (Pawn|GetControlRotation _returnvalue :!class /Script/Engine.Controller))
  (bind (_roll _pitch _yaw) (Math|Rotator|BreakRotator _returnvalue_2))
  (Pawn|SetControlRotation (Pawn|GetController (Variables|Default|GetCharacter)) (Math|Interpolation|RInterpTo _returnvalue_2 (Math|Rotator|MakeRotator Target%20X%20%28Roll%29 _pitch _yaw) (Utilities|Time|GetWorldDeltaSeconds) 1e+01)))

(fn WallRunJump
  (bind _wallrunnormal (Variables|Default|GetWallRunNormal))
  (bind _wallrunjumpoffforce (Variables|Default|GetWallRunJumpOffForce))
  (if (Variables|Default|GetWallRunning?)
    (CallFunction|WallRunEnd 0.35)
    (Character|LaunchCharacter (Variables|Default|GetCharacter) (Math|Vector|MakeVector (* _wallrunjumpoffforce (.x _wallrunnormal)) (* _wallrunjumpoffforce (.y _wallrunnormal)) (Variables|Default|GetWallRunJumpHeight)) false true)
    (return true)
    (else
      (return false))))