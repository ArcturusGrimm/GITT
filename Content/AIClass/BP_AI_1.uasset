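; BP_AI_1 is an AI character Blueprint built from modular Etasphera07 skeletal mesh parts.
; Its Construction Script sets the main Mesh as Master Pose Component for the head, body, arm, finger, leg and armor pieces.
; All parts follow the pose of that one mesh, so they animate together as a single body without separate animation logic.
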(fn ConstructionScript
  (Class|SkinnedMeshComponent|SetMasterPoseComponent (Variables|Default|GetSK_Etasphera07_Arm_thumb_02_r) (Variables|Default|GetMesh) false))