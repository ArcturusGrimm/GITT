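; Character Blueprint for Etasphera31, assembled from modular skeletal mesh parts covering body, head, plasma head, arms down to finger joints, legs and armor pieces.
; The construction script sets the main Mesh as master pose component for every part, so all pieces follow one skeleton's animation.
; It also attaches the Gun to the GripPoint socket on Mesh, snapping location and scale while keeping relative rotation.
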(fn ConstructionScript
  (Class|SkinnedMeshComponent|SetMasterPoseComponent (Variables|Default|GetSK_Etasphera31_Arm_thumb_03_r) (Variables|Character|GetMesh) false)
  (Transformation|AttachComponentToComponent (Variables|Default|GetGun) (Variables|Character|GetMesh) "GripPoint" "SnapToTarget" "KeepRelative" "SnapToTarget" true))