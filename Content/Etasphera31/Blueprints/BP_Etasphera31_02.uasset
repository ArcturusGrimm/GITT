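; Blueprint for Etasphera31 (variant 02), a modular robot-like character assembled from many separate skeletal mesh parts.
; Its construction script makes every arm, finger, leg, body, armor and plasma head component follow the main Mesh through SetMasterPoseComponent.
; The whole assembly therefore animates as one skeleton, driven by a single pose.
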(fn ConstructionScript
  (Class|SkinnedMeshComponent|SetMasterPoseComponent (Variables|Default|GetSK_Etasphera31_Arm_thumb_03_r) (Variables|Character|GetMesh)))